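; Trap actor that shoots arrows while the player character stands in its trigger volume.
; Trigger overlaps with ThirdPersonCharacter1 set and clear a flag, and entry also plays a wood creak sound at the trap.
; While the flag is set, Tick spawns a Flèche every frame at SpawnArraow's transform, with no cooldown.
; Each arrow's collision component receives an impulse equal to Detecteur's unscaled forward vector.
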(event `self.ReceiveTick`
  (params (DeltaSeconds :type "Float (single-precision)"))
  (if (`self.PlayerOnTrigger`)
    (bind _returnvalue (`|SpawnActorFromClass` "/Game/Blueprints/Projectiles/Flèche.Flèche_C" (`SceneComponent.K2_GetComponentToWorld` (`self.SpawnArraow`)) "Undefined" "OverrideRootScale" null null))
    (`PrimitiveComponent.AddImpulse` (`/Game/Blueprints/Projectiles/Flèche.CollisionComponent` _returnvalue) (`SceneComponent.GetForwardVector` (`self.Detecteur`)) "None" false)))

(event `self.Trigger.OnComponentBeginOverlap`
  (params (OverlappedComponent :type "PrimitiveComponent Object Reference") (OtherActor :type "Actor Object Reference") (OtherComp :type "PrimitiveComponent Object Reference") (OtherBodyIndex :type Integer) (bFromSweep :type Boolean) (SweepResult :type "HitResult Structure (by ref)"))
  (cast `/Game/ThirdPersonBP/Blueprints/ThirdPersonCharacter1` OtherActor)
  (`GameplayStatics.PlaySoundAtLocation` "/Game/Audios/woodcreak.woodcreak" (`self.K2_GetActorLocation`) (struct) 1.0 1.0 0.0 null null null)
  (set `self.PlayerOnTrigger` true))

(event `self.Trigger.OnComponentEndOverlap`
  (params (OverlappedComponent :type "PrimitiveComponent Object Reference") (OtherActor :type "Actor Object Reference") (OtherComp :type "PrimitiveComponent Object Reference") (OtherBodyIndex :type Integer))
  (cast `/Game/ThirdPersonBP/Blueprints/ThirdPersonCharacter1` OtherActor)
  (set `self.PlayerOnTrigger` false))

(fn `UserConstructionScript`)