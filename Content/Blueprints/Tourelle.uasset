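; Rotating four-barrel turret that fires continuously in volleys, turning between each one.
; On Tick, a DoOnce gates a sequence that spawns a ProjectileTourelle at each of the four spawn points.
; Every spawn feeds a shared chain of sound call and 0.4-second delay, after which the axis rotates 45 degrees and the DoOnce resets for the next volley.
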(event `self.ReceiveTick`
  (params (DeltaSeconds :type "Float (single-precision)"))
  ;[1 1 1] Tourelle rotationnelle à quatre canons
  (`/Engine/EditorBlueprintResources/StandardMacros.DoOnce` false :!label _label
    (:`Completed`
      (`|ExecutionSequence`
        (:`then_0`
          (`|SpawnActorFromClass` "/Game/Blueprints/Projectiles/ProjectileTourelle.ProjectileTourelle_C" (`SceneComponent.K2_GetComponentToWorld` (`self.Spawn1`)) "Undefined" "OverrideRootScale" null null))
        (:`then_1`
          (`|SpawnActorFromClass` "/Game/Blueprints/Projectiles/ProjectileTourelle.ProjectileTourelle_C" (`SceneComponent.K2_GetComponentToWorld` (`self.Spawn2`)) "Undefined" "OverrideRootScale" null null))
        (:`then_2`
          (`|SpawnActorFromClass` "/Game/Blueprints/Projectiles/ProjectileTourelle.ProjectileTourelle_C" (`SceneComponent.K2_GetComponentToWorld` (`self.Spawn3`)) "Undefined" "OverrideRootScale" null null))
        (:`then_3`
          (`|SpawnActorFromClass` "/Game/Blueprints/Projectiles/ProjectileTourelle.ProjectileTourelle_C" (`SceneComponent.K2_GetComponentToWorld` (`self.Spawn4`)) "Undefined" "OverrideRootScale" null null)))
      (if true
        (`GameplayStatics.PlaySoundAtLocation` null (0.0 0.0 0.0) (struct) 1.0 1.0 0.0 null null null)
        (`KismetSystemLibrary.Delay` 0.4)
        (`SceneComponent.K2_AddLocalRotation` (`self.Axe`) (struct :`Yaw` 45.0) false false)
        (goto _label :!via `Reset`)))))

(fn `UserConstructionScript`)