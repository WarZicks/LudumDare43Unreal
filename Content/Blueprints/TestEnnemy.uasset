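; TestEnnemy is a test enemy Blueprint that registers melee hits from the player's sword.
; When its Box overlaps a Weapon_Sword, it reads the ThirdPersonCharacter_Theo player's slash and heavy attack flags to print a simple or heavy hit message.
; An OnHit flag blocks repeat hits until a delay clears it, with a longer lockout for heavy hits.
; It only prints messages and applies no damage.
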(event `self.Box.OnComponentBeginOverlap`
  (params (OverlappedComponent :type "PrimitiveComponent Object Reference") (OtherActor :type "Actor Object Reference") (OtherComp :type "PrimitiveComponent Object Reference") (OtherBodyIndex :type Integer) (bFromSweep :type Boolean) (SweepResult :type "HitResult Structure (by ref)"))
  (bind _returnvalue (not (`self.onHit`)))
  (cast `/Game/Weapon_Sword` OtherActor)
  (bind _asthird_person_character_theo (cast `/Game/ThirdPersonBP/Blueprints/ThirdPersonCharacter_Theo` (`GameplayStatics.GetPlayerCharacter` 0)))
  (`|ExecutionSequence`
    (:`then_0`
      (if (and (`/Game/ThirdPersonBP/Blueprints/ThirdPersonCharacter_Theo.SlashSword` _asthird_person_character_theo) _returnvalue)
        (`KismetSystemLibrary.PrintString` "Simple Hit")
        (set `self.onHit` true)
        (`KismetSystemLibrary.Delay` 1.5)
        (set `self.onHit` false)))
    (:`then_1`
      (if (and _returnvalue (`/Game/ThirdPersonBP/Blueprints/ThirdPersonCharacter_Theo.HeavySwordAttack` _asthird_person_character_theo))
        (`KismetSystemLibrary.PrintString` "Heavy Hit")
        (set `self.onHit` true)
        (`KismetSystemLibrary.Delay` 2.5)
        (set `self.onHit` false)))))

(fn `UserConstructionScript`)